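; BP_StartWorld is an actor that drives the front-end menu flow from start screen to level menu.
; On BeginPlay it shows WBP_StartWorld and hands it a reference to itself.
; StartGame clears all widgets, then shows WBP_LevelMenu initialized with the map from GetFolderNameMap, which is not defined in this Blueprint.
; Destroying the actor triggers garbage collection.
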(event Custom|StartGame
  (Viewport|RemoveAllWidgets)
  (bind _returnvalue (UserInterface|CreateWidget "/Game/Blueprints/StartWorld/WBP_LevelMenu.WBP_LevelMenu_C"))
  (Default|Init _returnvalue (Class|StartActor|GetFolderNameMap))
  (UserInterface|Viewport|AddtoViewport _returnvalue 0))

(event EventBeginPlay
  (|CallParentFunction)
  (bind _returnvalue (UserInterface|CreateWidget "/Game/Blueprints/StartWorld/WBP_StartWorld.WBP_StartWorld_C"))
  (Variables|/Game/Blueprints/StartWorld/WBP_StartWorld.WBP_StartWorld_C|SetStartWorld _returnvalue self)
  (UserInterface|Viewport|AddtoViewport _returnvalue 0))

(event EventDestroyed
  (Utilities|Platform|CollectGarbage))

(fn ConstructionScript)